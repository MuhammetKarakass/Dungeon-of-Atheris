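; GA_Firebolt is a gameplay ability that casts homing firebolts at the location or actor under the mouse.
; On activation it commits, gets cursor target data, turns the caster toward the hit location through CombatInterface and plays the cast montage.
; A montage gameplay event triggers SpawnProjectiles from the weapon socket with an overridden pitch, passing the hit actor as homing target.
; The ability ends when the montage completes, blends out, or is interrupted or cancelled.
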(event Ability|EventActivateAbility
  (Ability|CommitAbility)
  (bind _datahandle (|TargetDataUnderMouse)
    (:ValidData
      (Variables|Default|SetProjectile%20Target%20Location (.location (Ability|TargetData|GetHitResultfromTargetData _datahandle)))
      (Variables|Default|SetMouseHitActor (.hitactor (Ability|TargetData|GetHitResultfromTargetData _datahandle)))
      (bind _ascombat_interface (Utilities|Casting|CastToCombatInterface (Ability|GetAvatarActorfromActorInfo)))
      (Class|CombatInterface|UpdateFacingTarget _ascombat_interface (Variables|Default|GetProjectile%20Target%20Location))
      (|PlayMontageandWaitProxy "None" "/Game/Assets/Characters/Aura/Animations/Abilities/AM_Cast_Firebolt.AM_Cast_Firebolt" 1.0 "None" false 1.0 0.0 false
        (:then
          (Ability|Tasks|WaitGameplayEvent "(TagName=\"Event.Montage.FireBolt\")" 0
            (:EventReceived
              (Class|AuraFireBoltAbility|SpawnProjectiles (Variables|Default|GetProjectile%20Target%20Location) (GameplayTags|MakeLiteralGameplayTag "(TagName=\"CombatSocket.Weapon\")") true 45.0 (Variables|Default|GetMouseHitActor)))))
        (:OnCompleted
          (Ability|EndAbility :!label _label))
        (:OnBlendOut
          (goto _label))
        (:OnInterrupted
          (goto _label))
        (:OnCancelled
          (goto _label))))))

(event Ability|EventOnEndAbility
  (params (bWasCancelled :type Boolean)))