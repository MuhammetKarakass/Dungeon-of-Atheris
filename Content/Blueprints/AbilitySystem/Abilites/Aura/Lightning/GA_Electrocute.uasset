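; Channeled lightning ability that locks the caster in place and shocks the target under the cursor plus additional chained targets.
; A montage event starts the beam trace and ShockLoop gameplay cues, attached from weapon to primary target, then to the others.
; A looping timer commits cost and applies lightning damage until cost fails.
; Input release, after a minimum-time delay, also triggers cleanup, final damage effects and cooldown, as does primary target death.
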(event Custom|DamageAndCost
  (bind _returnvalue (Ability|CommitAbilityCost false))
  (if _returnvalue
    (CallFunction|ApplyDamage)
    (else
      (CallFunction|ClearTimeEndAbility))))

(event Ability|EventActivateAbility
  (if (Utilities|DoesObjectImplementInterface (Ability|GetAvatarActorfromActorInfo) "/Script/DungeonOfAtheris.CombatInterface")
    (bind _datahandle (|TargetDataUnderMouse)
      (:ValidData
        (Class|AuraBeamSpell|StoreMouseDataInfo (Ability|TargetData|GetHitResultfromTargetData _datahandle))
        (Class|AuraBeamSpell|StoreOwnerVariables)
        (Utilities|FlowControl|Sequence
          (:then_0
            (Variables|/Script/Engine.PlayerController|SetbShowMouseCursor (Variables|Default|GetOwnerPlayerController) false)
            (Class|CombatInterface|UpdateFacingTarget(Message) (Ability|GetAvatarActorfromActorInfo) (Variables|Default|GetMouseHitLocation))
            (GameplayCue|ExecuteGameplayCue :GameplayCueTag "(TagName=\"GameplayCue.ShockBurst\")")
            (|PlayMontageandWaitProxy "None" (Variables|Default|GetMontage_Electrocute) 1.0 "None" true 1.0 0.0 false
              (:then
                (Ability|Tasks|WaitGameplayEvent "(TagName=\"Event.Montage.Electrocute\")" 0
                  (:then
                    (Class|CombatInterface|SetinShockLoop(Message) (Ability|GetAvatarActorfromActorInfo) true)
                    (Pawn|Components|CharacterMovement|DisableMovement (Variables|/Script/Engine.Character|GetCharacterMovement (Variables|Default|GetOwnerCharacter)))
                    (Class|AuraBeamSpell|TraceFirstTarget (Variables|Default|GetMouseHitLocation))
                    (bind _returnvalue (Class|CombatInterface|GetWeapon(Message) (Variables|Default|GetOwnerCharacter)))
                    (Variables|Default|SetFirtsTargetCueParams (Ability|GameplayCue|MakeGameplayCueParameters :Location (Variables|Default|GetMouseHitLocation) :SourceObject (Variables|Default|GetMouseHitActor) :TargetAttachComponent _returnvalue))
                    (bind _output_get (Variables|Default|SetFirtsTargetImplementsInterface (Utilities|DoesObjectImplementInterface (Variables|Default|GetMouseHitActor) "/Script/DungeonOfAtheris.CombatInterface")))
                    (if _output_get
                      (Variables|Default|SetCueTarget (Variables|Default|GetMouseHitActor))
                      (else
                        (Variables|Default|SetCueTarget (Ability|GetAvatarActorfromActorInfo))))
                    (GameplayCue|AddGameplayCueOnActor(Looping) (Variables|Default|GetCueTarget) "(TagName=\"GameplayCue.ShockLoop\")" (Variables|Default|GetFirtsTargetCueParams))
                    (if (Variables|Default|GetFirtsTargetImplementsInterface)
                      (Class|CombatInterface|SetIsBeingShocked(Message) (Variables|Default|GetCueTarget) true)
                      (bind _outadditionaltargets (Class|AuraBeamSpell|StoreAdditionalTargets))
                      (bind _output_get_2 (Variables|Default|SetOut%20Additional%20Targets _outadditionaltargets))
                      (for _array_element _output_get_2
                        (Class|CombatInterface|SetIsBeingShocked(Message) _array_element true)
                        (CallFunction|AddShockLoopCuetoAdditionalTarget _array_element)
                        (bind _returnvalue_2 (Utilities|Time|SetTimerbyEvent (delegate Custom|DamageAndCost) (Variables|Default|GetDamageDeltaTime) true))
                        (Variables|Default|SetSetDamageAndCostTimer _returnvalue_2))))))))
          (:then_1
            (bind _timeheld (Ability|Tasks|WaitInputRelease false)
              (:OnRelease
                (bind _output_get_3 (Variables|Default|SetTime%20Held _timeheld))
                (if true
                  (Utilities|FlowControl|Delay (- (Variables|Default|GetMinSpellTime) (Variables|Default|GetTime%20Held))))
                (CallFunction|ClearTimeEndAbility)))))))
    (else
      (Ability|EndAbility))))

(event Ability|EventOnEndAbility
  (params (bWasCancelled :type Boolean)))

(event EventPrimaryTargetDied
  (params (DeadActor :type Actor%20Object%20Reference))
  (GameplayCue|RemoveGameplayCueOnActor(Looping) DeadActor "(TagName=\"GameplayCue.ShockLoop\")" (Variables|Default|GetFirtsTargetCueParams))
  (CallFunction|ClearTimeEndAbility))

(event EventAdditionalTargetDied
  (params (DeadActor :type Actor%20Object%20Reference))
  (CallFunction|RemoveShockLoopCuefromAdditionalTarget DeadActor)
  (Utilities|Array|RemoveItem (Variables|Default|GetOut%20Additional%20Targets) DeadActor))

(fn AddShockLoopCuetoAdditionalTarget
  (params (AdditionalTarget :type Actor%20Object%20Reference))
  (LocalVariables|SetTargetActor AdditionalTarget)
  (Utilities|Map|Add (Variables|Default|GetAdditionalActorToCueParamas) (LocalVariables|GetTargetActor) (Ability|GameplayCue|MakeGameplayCueParameters :Location (Transformation|GetActorLocation (LocalVariables|GetTargetActor)) :SourceObject (LocalVariables|GetTargetActor) :TargetAttachComponent (Variables|/Script/Engine.Actor|GetRootComponent (Variables|Default|GetMouseHitActor))))
  (GameplayCue|AddGameplayCueOnActor(Looping) (LocalVariables|GetTargetActor) "(TagName=\"GameplayCue.ShockLoop\")" (Ability|GameplayCue|MakeGameplayCueParameters :Location (Transformation|GetActorLocation (LocalVariables|GetTargetActor)) :SourceObject (LocalVariables|GetTargetActor) :TargetAttachComponent (Variables|/Script/Engine.Actor|GetRootComponent (Variables|Default|GetMouseHitActor)))))

(fn PrepareEndAbility
  (bind _mousehitactor (Variables|Default|GetMouseHitActor))
  (Variables|/Script/Engine.PlayerController|SetbShowMouseCursor (Variables|Default|GetOwnerPlayerController) true)
  (Class|CombatInterface|SetinShockLoop(Message) (Ability|GetAvatarActorfromActorInfo) false)
  (Pawn|Components|CharacterMovement|SetMovementMode (Variables|/Script/Engine.Character|GetCharacterMovement (Variables|Default|GetOwnerCharacter)) "MOVE_Walking" 0)
  (if (Variables|Default|GetFirtsTargetImplementsInterface)
    (Class|CombatInterface|SetIsBeingShocked(Message) (Variables|Default|GetMouseHitActor) false)
    (GameplayCue|RemoveGameplayCueOnActor(Looping) _mousehitactor "(TagName=\"GameplayCue.ShockLoop\")" (Variables|Default|GetFirtsTargetCueParams))
    (Class|AuraAbilitySystemLibrary|ApplyDamageEffect (Class|DamageGameplayAbility|MakeDamageEffectParamsfromClassDefaults _mousehitactor))
    (for _array_element (Variables|Default|GetOut%20Additional%20Targets)
      (Class|CombatInterface|SetIsBeingShocked(Message) _array_element false)
      (CallFunction|RemoveShockLoopCuefromAdditionalTarget _array_element)
      (Class|AuraAbilitySystemLibrary|ApplyDamageEffect (Class|DamageGameplayAbility|MakeDamageEffectParamsfromClassDefaults _array_element)))
    (else
      (GameplayCue|RemoveGameplayCueOnActor(Looping) (Ability|GetAvatarActorfromActorInfo) "(TagName=\"GameplayCue.ShockLoop\")" (Variables|Default|GetFirtsTargetCueParams)))))

(fn ApplyDamage
  (CallFunction|ApplyDamageSingleTarget (Variables|Default|GetMouseHitActor))
  (for _array_element (Variables|Default|GetOut%20Additional%20Targets)
    (CallFunction|ApplyDamageSingleTarget _array_element)))

(fn ApplyDamageSingleTarget
  (params (Actor :type Actor%20Object%20Reference))
  (bind _returnvalue (Ability|GetAbilitySystemComponentfromActorInfo))
  (Utilities|IsValid _returnvalue
    (:Is%20Valid
      (bind _returnvalue_2 (Ability|GameplayEffect|AssignTagSetbyCallerMagnitude (GameplayEffects|MakeOutgoingSpec _returnvalue (Variables|Default|GetDamageEffectClass) (Math|Conversions|ToFloat(Integer) (Ability|GetAbilityLevel)) (GameplayEffects|MakeEffectContext _returnvalue)) "(TagName=\"Damage.Lightning\")" (Class|DamageGameplayAbility|GetDamageatLevel)))
      (GameplayEffects|ApplyGameplayEffectSpecToSelf (Ability|GetAbilitySystemComponent Actor) _returnvalue_2))))

(fn RemoveShockLoopCuefromAdditionalTarget
  (params (Target :type Actor%20Object%20Reference))
  (Variables|Default|SetTargett Target)
  (if (.ReturnValue (Utilities|Map|Find (Variables|Default|GetAdditionalActorToCueParamas) (Variables|Default|GetTargett)))
    (GameplayCue|RemoveGameplayCueOnActor(Looping) (Variables|Default|GetTargett) "(TagName=\"GameplayCue.ShockLoop\")" (.Value (Utilities|Map|Find (Variables|Default|GetAdditionalActorToCueParamas) (Variables|Default|GetTargett))))))

(fn ClearTimeEndAbility
  (Utilities|Time|ClearandInvalidateTimerbyHandle (Variables|Default|GetSetDamageAndCostTimer))
  (CallFunction|PrepareEndAbility)
  (Ability|CommitAbilityCooldown false)
  (Utilities|Array|Clear (Variables|Default|GetOut%20Additional%20Targets))
  (Utilities|Map|Clear (Variables|Default|GetAdditionalActorToCueParamas))
  (Variables|Default|SetMouseHitActor 0)
  (Variables|Default|SetFirtsTargetImplementsInterface false)
  (Variables|Default|SetTime%20Held 0.0)
  (Ability|EndAbility))