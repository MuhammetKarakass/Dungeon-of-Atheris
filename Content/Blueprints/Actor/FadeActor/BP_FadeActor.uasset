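; BP_FadeActor is a static mesh actor that fades out and back in when its FadeOut and Fadein events are called.
; Construction caches original materials and builds dynamic instances from fade materials, which FadeOut applies before a timeline drives their "Fade" parameter.
; Near-zero fade makes the mesh ignore a custom trace channel, plus Visibility when BlockVisibility is set.
; Reversing to full fade value restores original materials and blocking.
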(event EventBeginPlay)

(event Collision|EventActorBeginOverlap
  (params (OtherActor :type Actor%20Object%20Reference)))

(event EventTick
  (params (DeltaSeconds :type Float%20%28single-precision%29)))

(event EventFadeOut
  (CallFunction|SetMaterialstoDynamicInstances)
  (bind _fade (Timeline|FadeTimeline Play)
    (:Update
      (for _array_element (Variables|Default|GetDynmaicMaterialInstances)
        (Rendering|Material|SetScalarParameterValue _array_element "Fade" _fade :!class /Script/Engine.MaterialInstanceDynamic)))
    (:Finished
      (if (>= _fade 1.0)
        (for (_array_element_2 _array_index) (Variables|Default|GetOriginalMaterials)
          (Rendering|Material|SetMaterial (Variables|Default|GetStaticMesh) _array_index _array_element_2)
          (Collision|SetCollisionResponsetoChannel (Variables|Default|GetStaticMesh) "ECC_GameTraceChannel2" "ECR_Block")
          (if (Variables|Default|GetBlockVisibility)
            (Collision|SetCollisionResponsetoChannel (Variables|Default|GetStaticMesh) "ECC_Visibility" "ECR_Block")))
        (elif (<= _fade 0.2)
          (Collision|SetCollisionResponsetoChannel (Variables|Default|GetStaticMesh) "ECC_GameTraceChannel2" "ECR_Ignore")
          (if (Variables|Default|GetBlockVisibility)
            (Collision|SetCollisionResponsetoChannel (Variables|Default|GetStaticMesh) "ECC_Visibility" "ECR_Ignore")))))))

(event EventFadein
  (bind _fade (Timeline|FadeTimeline Reverse)
    (:Update
      (for _array_element (Variables|Default|GetDynmaicMaterialInstances)
        (Rendering|Material|SetScalarParameterValue _array_element "Fade" _fade :!class /Script/Engine.MaterialInstanceDynamic)))
    (:Finished
      (if (>= _fade 1.0)
        (for (_array_element_2 _array_index) (Variables|Default|GetOriginalMaterials)
          (Rendering|Material|SetMaterial (Variables|Default|GetStaticMesh) _array_index _array_element_2)
          (Collision|SetCollisionResponsetoChannel (Variables|Default|GetStaticMesh) "ECC_GameTraceChannel2" "ECR_Block")
          (if (Variables|Default|GetBlockVisibility)
            (Collision|SetCollisionResponsetoChannel (Variables|Default|GetStaticMesh) "ECC_Visibility" "ECR_Block")))
        (elif (<= _fade 0.2)
          (Collision|SetCollisionResponsetoChannel (Variables|Default|GetStaticMesh) "ECC_GameTraceChannel2" "ECR_Ignore")
          (if (Variables|Default|GetBlockVisibility)
            (Collision|SetCollisionResponsetoChannel (Variables|Default|GetStaticMesh) "ECC_Visibility" "ECR_Ignore")))))))

(fn ConstructionScript
  (Utilities|Array|Clear (Variables|Default|GetDynmaicMaterialInstances))
  (Variables|Default|SetOriginalMaterials (Rendering|Material|GetMaterials (Variables|Default|GetStaticMesh)))
  (for _array_element (Variables|Default|GetFadeMaterialInstances)
    (bind _returnvalue (Rendering|Material|CreateDynamicMaterialInstance _array_element "None" "None" :!class /Script/Engine.KismetMaterialLibrary))
    (Utilities|Array|AddUnique (Variables|Default|GetDynmaicMaterialInstances) _returnvalue)))

(fn SetMaterialstoDynamicInstances
  (for (_array_element _array_index) (Variables|Default|GetDynmaicMaterialInstances)
    (Rendering|Material|SetMaterial (Variables|Default|GetStaticMesh) _array_index _array_element)))