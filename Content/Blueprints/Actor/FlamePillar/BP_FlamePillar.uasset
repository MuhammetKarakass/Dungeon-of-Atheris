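; BP_FlamePillar is a flame pillar actor whose point light flickers continuously.
; On BeginPlay it randomly picks one of two flame intensity timelines and plays it from the start, then picks again whenever one finishes.
; Each timeline update passes its curve value to UpdateLightIntensity, which scales it by BaseIntensity and applies it to the PointLight.
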(event Custom|Start_Timline_2
  (bind _flameintensity (Timeline|Flame%20Intensity%20Timeline_2 PlayFromStart)
    (:Update
      (CallFunction|UpdateLightIntensity _flameintensity))
    (:Finished
      (CallFunction|ChooseTimeline))))

(event Custom|Start_Timline_1
  (bind _flameintensity (Timeline|Flame%20Intensity%20Timeline_1 PlayFromStart)
    (:Update
      (CallFunction|UpdateLightIntensity _flameintensity))
    (:Finished
      (CallFunction|ChooseTimeline))))

(event Custom|Choose_Timeline
  (switch int (Math|Random|RandomIntegerinRange 0 1)
    (:Default
      (CallFunction|StartTimline2 :!label _label))
    (:0
      (CallFunction|StartTimline1))
    (:1
      (goto _label))))

(event EventBeginPlay
  (CallFunction|ChooseTimeline))

(fn ConstructionScript)

(fn UpdateLightIntensity
  (params (Intensity :type Float%20%28double-precision%29))
  (Rendering|Components|Light|SetIntensity (Variables|Default|GetPointLight) (* Intensity (Variables|Default|GetBaseIntensity))))