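; BP_MapEntranceStair is a map entrance stair actor in the Checkpoint folder that can be highlighted with lights.
; HiglightActor shows its two point lights and UnHiglightActor hides them, without propagating visibility to child components.
; It has no other logic of its own: BeginPlay and Tick are disabled, and the construction script only calls its parent.
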(event EventBeginPlay
  (|CallParentFunction) ; This node is disabled and will not be called.\nDrag off pins to build functionality.
)

(event EventTick
  (params (DeltaSeconds :type Float%20%28single-precision%29))
  (|CallParentFunction DeltaSeconds) ; This node is disabled and will not be called.\nDrag off pins to build functionality.
)

(event EventHiglightActor
  (Rendering|SetVisibility (Variables|Default|GetPointLight) true false))

(event EventUnHiglightActor
  (Rendering|SetVisibility (Variables|Default|GetPointLight) false false))

(fn ConstructionScript
  (|CallParentFunction))