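; Base enemy character Blueprint that handles spawn, facing and dissolve presentation.
; On BeginPlay, a timeline uniformly scales the mesh for a spawn effect.
; UpdateFacingTarget feeds a location to Motion Warping as the FacingTarget warp target.
; Separate mesh and weapon events take dynamic materials and drive their Dissolve parameter through their own timelines.
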(event EventBeginPlay
  (bind _spawn (Timeline|Spawn%20TimeLine Play)
    (:Update
      (Transformation|SetRelativeScale3D (Variables|Character|GetMesh) (Math|Vector|MakeVector _spawn _spawn _spawn)))))

(event Collision|EventActorBeginOverlap
  (params (OtherActor :type Actor%20Object%20Reference)))

(event EventTick
  (params (DeltaSeconds :type Float%20%28single-precision%29)))

(event EventMeshStartDissolveTimer
  (params (DynamicMaterialDynamic :type Material%20Instance%20Dynamic%20Object%20Reference))
  (bind _meshdisolvetrack (Timeline|MeshDisolveTimeline Play)
    (:Update
      (Rendering|Material|SetScalarParameterValue DynamicMaterialDynamic "Dissolve" _meshdisolvetrack :!class /Script/Engine.MaterialInstanceDynamic))))

(event EventWeaponStartDissolveTimer
  (params (DynamicMaterialDynamic :type Material%20Instance%20Dynamic%20Object%20Reference))
  (bind _weapondisolvetrack (Timeline|WeaponDisolveTimeLine Play)
    (:Update
      (Rendering|Material|SetScalarParameterValue DynamicMaterialDynamic "Dissolve" _weapondisolvetrack :!class /Script/Engine.MaterialInstanceDynamic))))

(event EventUpdateFacingTarget
  (params (Target :type Vector%20%28by%20ref%29 :default "0, 0, 0"))
  (Class|MotionWarpingComponent|AddorUpdateWarpTargetfromLocation (Variables|Default|GetMotionWarping) "FacingTarget" Target))

(fn ConstructionScript)